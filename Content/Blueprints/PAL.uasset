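; PAL is an actor that travels along a referenced spline while turning to face a fixed world point, with a yaw offset.
; Each Tick advances the spline distance by a fixed step, so speed depends on frame rate.
; It detects the spline's end when its position stops changing between ticks, then resets the distance to loop from the start.
; The player pawn is cached on BeginPlay but not used.
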(event EventTick
  (params (DeltaSeconds :type Float%20%28single-precision%29))
  (bind _returnvalue (Math|Vector|MakeVector -5.03e+03 -1629.0 1.11e+03))
  (bind _returnvalue_2 (Transformation|GetActorLocation))
  (bind _returnvalue_3 (Transformation|GetActorLocation))
  (bind _returnvalue_4 (Math|Rotator|FindLookatRotation _returnvalue_2 _returnvalue))
  (bind (_roll _pitch _yaw) (Math|Rotator|BreakRotator _returnvalue_4))
  (Transformation|SetActorLocation (Spline|GetLocationatDistanceAlongSpline (Variables|/Game/Blueprints/SplineBP.SplineBP_C|GetSpline (Variables|Default|GetSpline)) (Variables|Default|GetSplineDistance) "World") false false)
  (Transformation|SetActorRotation (Math|Rotator|MakeRotator _roll _pitch (+ _yaw -9e+01)))
  (Variables|Default|SetSplineDistance (+ (Variables|Default|GetSplineDistance) 5.0))
  (if (Variables|Default|GetStarted)
    (if (Math|Vector|Equal(Vector) (Variables|Default|GetLocationLastTick) _returnvalue_3 1.0)
      (Variables|Default|SetSplineDistance 0.0)
      (Variables|Default|SetStarted false)
      (else
        (Variables|Default|SetLocationLastTick _returnvalue_3 :!label _label)))
    (else
      (Variables|Default|SetStarted true)
      (Variables|Default|SetSplineDistance (+ (Variables|Default|GetSplineDistance) 5.0))
      (goto _label))))

(event EventBeginPlay
  (Variables|Default|SetPlayer (Game|Player|GetPlayerPawn 0))
  (Variables|Default|SetLocationLastTick (Transformation|GetActorLocation)))

(fn ConstructionScript)