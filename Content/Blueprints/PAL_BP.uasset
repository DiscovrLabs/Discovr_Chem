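; PAL actor whose mouth material glows green in time with an audio clip, presumably its speech.
; BeginPlay creates a dynamic material on the mesh's second slot.
; Tick samples the SoundWave's frequency spectrum at the time elapsed since AudioStartTime, mapping the clamped single band to emissive green intensity.
; Paired DoOnce gates black out the mouth once after each clip's duration ends.
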(event EventBeginPlay
  (bind _returnvalue (Rendering|Material|CreateDynamicMaterialInstance (Variables|Default|GetStaticMesh) 1 0 :!class /Script/Engine.PrimitiveComponent))
  (Variables|Default|SetMouthMat _returnvalue))

(event EventTick
  (params (DeltaSeconds :type Float%20%28single-precision%29))
  (bind _returnvalue (Utilities|Time|GetGameTimeinSeconds))
  (bind _clip (Variables|Default|GetClip))
  (bind _audiostarttime (Variables|Default|GetAudioStartTime))
  (bind _returnvalue_2 (- _returnvalue _audiostarttime))
  (if (Utilities|IsValid _clip)
    (if (<= _returnvalue_2 (Variables|/Script/Engine.SoundBase|GetDuration _clip))
      (bind _assound_wave (Utilities|Casting|CastToSoundWave _clip))
      (bind _outspectrum (Class|SoundVisualizationStatics|CalculateFrequencySpectrum _assound_wave 0 _returnvalue_2 0.01 1))
      (Rendering|Material|SetVectorParameterValue (Variables|Default|GetMouthMat) "Emmissive Color" (Utilities|Struct|MakeLinearColor 0.0 (Math|Float|MapRangeUnclamped (Math|Float|Clamp(Float) (Utilities|Array|Get(acopy) _outspectrum) -2e+01 35.0) -2e+01 35.0 0.0 1.0) 0.0 1.0) :!class /Script/Engine.MaterialInstanceDynamic)
      (Utilities|FlowControl|DoOnce false :!label _label
        (:Completed
          (goto _label_2 Reset)))
      (else
        (Utilities|FlowControl|DoOnce false :!label _label_2
          (:Completed
            (Rendering|Material|SetVectorParameterValue (Variables|Default|GetMouthMat) "Emmissive Color" (Utilities|Struct|MakeLinearColor 0.0 0.0 0.0 1.0) :!class /Script/Engine.MaterialInstanceDynamic)
            (goto _label Reset)))))))

(fn ConstructionScript)