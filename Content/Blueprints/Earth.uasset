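; Earth is an actor that spins continuously and removes itself based on the player's position.
; Each tick it adds yaw rotation scaled by RotationSpeed and frame time.
; It then destroys itself once the first player pawn's world Y drops below its own Y plus a fixed offset.
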(event EventTick
  (params (DeltaSeconds :type Float%20%28single-precision%29))
  (Class|Actor|AddActorWorldRotation (Math|Rotator|MakeRotator 0.0 0.0 (* DeltaSeconds (Variables|Default|GetRotationSpeed))))
  (if (< (.Y (Math|Vector|BreakVector (Transformation|GetActorLocation (Game|Player|GetPlayerPawn 0)))) (+ (.Y (Math|Vector|BreakVector (Transformation|GetActorLocation))) 4.5e+02))
    (Actor|DestroyActor)))

(fn ConstructionScript)